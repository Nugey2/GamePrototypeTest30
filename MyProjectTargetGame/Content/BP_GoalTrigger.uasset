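; BP_GoalTrigger is a goal trigger volume that detects when a BP_Football enters it and scores a goal.
; On overlap it increments the Goals counter on BP_FirstPersonGameMode and prints a debug message.
; It then destroys the ball and spawns a fresh BP_Football at a hard-coded world location to reset play.
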(event OnComponentBeginOverlap(GoalTrigger)
  (params (OverlappedComponent :type Primitive%20Component%20Object%20Reference) (OtherActor :type Actor%20Object%20Reference) (OtherComp :type Primitive%20Component%20Object%20Reference) (OtherBodyIndex :type Integer) (bFromSweep :type Boolean) (SweepResult :type Hit%20Result%20Structure%20%28by%20ref%29))
  (Utilities|Casting|CastToBP_Football OtherActor)
  (bind _asbp_first_person_game_mode (Utilities|Casting|CastToBP_FirstPersonGameMode (Game|GetGameMode)))
  (Variables|/Game/FirstPerson/Blueprints/BP_FirstPersonGameMode.BP_FirstPersonGameMode_C|SetGoals _asbp_first_person_game_mode (+ (Variables|/Game/FirstPerson/Blueprints/BP_FirstPersonGameMode.BP_FirstPersonGameMode_C|GetGoals _asbp_first_person_game_mode) 1))
  (Development|PrintString "Goal Scored")
  (bind _asbp_football (Utilities|Casting|CastToBP_Football OtherActor))
  (Actor|DestroyActor _asbp_football)
  (Game|SpawnActorfromClass "/Game/BP_Football.BP_Football_C" (Math|Transform|MakeTransform "-1852.494597,-6704.202417,138.006565") "Undefined" "MultiplyWithRoot" 0 0))

(event EventBeginPlay)

(event Collision|EventActorBeginOverlap
  (params (OtherActor :type Actor%20Object%20Reference)))

(event EventTick
  (params (DeltaSeconds :type Float%20%28single-precision%29)))

(fn ConstructionScript)
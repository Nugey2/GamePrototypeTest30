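; BP_KillBox is a trigger volume that destroys and respawns the player or the football when either overlaps its box.
; A first-person character is destroyed after a short delay, then the game mode restarts player controller 0.
; A football is destroyed immediately and a new one spawns at a hardcoded world location.
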(event OnComponentBeginOverlap(Box)
  (params (OverlappedComponent :type Primitive%20Component%20Object%20Reference) (OtherActor :type Actor%20Object%20Reference) (OtherComp :type Primitive%20Component%20Object%20Reference) (OtherBodyIndex :type Integer) (bFromSweep :type Boolean) (SweepResult :type Hit%20Result%20Structure%20%28by%20ref%29))
  (Utilities|FlowControl|Sequence
    (:then_0
      (bind _asbp_first_person_character (Utilities|Casting|CastToBP_FirstPersonCharacter OtherActor))
      (Utilities|FlowControl|Delay 1.0)
      (Actor|DestroyActor _asbp_first_person_character)
      (Class|GameModeBase|RestartPlayer (Game|GetGameMode) (Game|GetPlayerController 0)))
    (:then_1
      (bind _asbp_football (Utilities|Casting|CastToBP_Football OtherActor))
      (Actor|DestroyActor _asbp_football)
      (Game|SpawnActorfromClass "/Game/BluePrintClasses/BP_Football.BP_Football_C" (Math|Transform|MakeTransform "-1852.494597,-6704.202417,138.006565") "Undefined" "MultiplyWithRoot" 0 0))))

(event EventBeginPlay)

(event Collision|EventActorBeginOverlap
  (params (OtherActor :type Actor%20Object%20Reference)))

(event EventTick
  (params (DeltaSeconds :type Float%20%28single-precision%29)))

(fn ConstructionScript)